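; Test tube trigger that reveals a second tube when a BP_test_tube actor first overlaps it.
; The overlap passes a DoOnce, scans all actors for BP_test_tube1 instances tagged "test", shows their mesh, blood and cap, and plays the Udar 2D sound for each.
; BeginPlay looks up "blood"-tagged tubes without acting on them, and a leftover teleport of the tube is disconnected.
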(event OnComponentBeginOverlap(Capsule)
  (params (OverlappedComponent :type Primitive%20Component%20Object%20Reference) (OtherActor :type Actor%20Object%20Reference) (OtherComp :type Primitive%20Component%20Object%20Reference) (OtherBodyIndex :type Integer) (bFromSweep :type Boolean) (SweepResult :type Hit%20Result%20Structure%20%28by%20ref%29)))

(event EventBeginPlay
  (bind _outactors (Actor|GetAllActorsOfClass "/Script/Engine.Actor"))
  (for _array_element _outactors
    (if (Actor|ActorHasTag _array_element "blood")
      (bind _asbp_test_tube (Utilities|Casting|CastToBP_test_tube _array_element)))))

(event Collision|EventActorBeginOverlap
  (params (OtherActor :type Actor%20Object%20Reference))
  (Utilities|Casting|CastToBP_test_tube OtherActor)
  (Utilities|FlowControl|DoOnce false
    (:Completed
      (bind _outactors (Actor|GetAllActorsOfClass "/Script/Engine.Actor"))
      (for _array_element _outactors
        (if (Actor|ActorHasTag _array_element "test")
          (bind _asbp_test_tube_1 (Utilities|Casting|CastToBP_test_tube1 _array_element))
          (Rendering|SetVisibility (Variables|/Script/Engine.StaticMeshActor|GetStaticMeshComponent _asbp_test_tube_1) true false)
          (Rendering|SetVisibility (Variables|/Game/morg/BP/BP_test_tube1.BP_test_tube1_C|Getblood%201 _asbp_test_tube_1) true false)
          (Rendering|SetVisibility (Variables|/Game/morg/BP/BP_test_tube1.BP_test_tube1_C|Getcap%201 _asbp_test_tube_1) true false)
          (Audio|SpawnSound2D "/Game/morg/sounds/zvyki/udar.udar" 1.0 1.0 0.0 0))))))

(event EventTick
  (params (DeltaSeconds :type Float%20%28single-precision%29)))

(fn ConstructionScript)