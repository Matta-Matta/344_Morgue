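; BP_probirka_tp1 is an overlap-triggered actor in the morgue content that hides test tubes.
; When any actor begins overlapping it, it scans every actor in the level for the "tube" tag and casts matches to BP_test_tube.
; Each tube's static mesh, cap and blood components are made invisible, regardless of which actor overlapped.
; An unconnected DoOnce branch that would move a tube to a fixed location never runs.
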(event EventBeginPlay)

(event Collision|EventActorBeginOverlap
  (params (OtherActor :type Actor%20Object%20Reference))
  (bind _outactors (Actor|GetAllActorsOfClass "/Script/Engine.Actor"))
  (for _array_element _outactors
    (if (Actor|ActorHasTag _array_element "tube")
      (bind _asbp_test_tube (Utilities|Casting|CastToBP_test_tube _array_element))
      (Rendering|SetVisibility (Variables|/Script/Engine.StaticMeshActor|GetStaticMeshComponent _asbp_test_tube) false false)
      (Rendering|SetVisibility (Variables|/Game/morg/BP/BP_test_tube.BP_test_tube_C|Getcap _asbp_test_tube) false false)
      (Rendering|SetVisibility (Variables|/Game/morg/BP/BP_test_tube.BP_test_tube_C|Getblood _asbp_test_tube) false false))))

(event EventTick
  (params (DeltaSeconds :type Float%20%28single-precision%29)))

(fn ConstructionScript)